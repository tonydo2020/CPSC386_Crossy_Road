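; Player chicken character for a Crossy Road-style game, handling hop movement, death and the title, score and death UI.
; Input checks death, bounds and mid-jump state, turns the mesh, then runs timelines that jump and offset the capsule; forward hops raise distance.
; Vehicle or river hits, or 600 idle ticks (eagle spawn is stubbed), trigger death with flattened mesh and sound.
; While alive, Tick nudges the spring arm after the chicken.
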(event OnComponentHit(StaticMesh)
  (params (HitComponent :type Primitive%20Component%20Object%20Reference) (OtherActor :type Actor%20Object%20Reference) (OtherComp :type Primitive%20Component%20Object%20Reference) (NormalImpulse :type Vector :default "0, 0, 0") (Hit :type Hit%20Result%20Structure%20%28by%20ref%29))
  ;[1 1 1] Get/Set Chicken Death
  (if (Variables|Default|GetIsDead)
    (Variables|Default|SetIsDead true)
    (else
      (Utilities|Casting|CastToRiver_Blueprint OtherActor)
      (Variables|Default|SetIsDead true)
      (Variables|Default|SetIsDrownDeath true))))

(event EventTick
  (params (DeltaSeconds :type Float%20%28single-precision%29))
  (bind _capsulecomponent (Variables|Collision|GetCapsuleComponent))
  (bind _staticmesh (Variables|Default|GetStaticMesh))
  (bind _staticmesh_2 (Variables|Default|GetStaticMesh))
  (bind _returnvalue (Transformation|GetWorldLocation _staticmesh_2))
  (bind _returnvalue_2 (Transformation|GetWorldRotation _capsulecomponent))
  ;[1 1 1] Chicken Movement
  (bind _result (Math|Integer|IncrementInt (Variables|Default|GetIdleTime))
    (:%20%20
      (if (== _result 600)
        (Variables|Default|SetIsDead true)
        (Variables|Default|SetIsEagleDeath true))
      (CallFunction|IstheChickenMid-Jump)
      (if (or (Variables|Default|GetisBlockedLeft) (Variables|Default|GetisBlockedRight))
        (CallFunction|PutChickenBackinBounds))
      ;[1 1 1] Chicken Death Result
      (if (Variables|Default|GetIsDead)
        (Variables|Default|SetGameStart false)
        (if (Variables|Default|GetDeathSoundPlayed)
          _
          (else
            (CallFunction|PlayDeathSound)
            (Variables|Default|SetDeathSoundPlayed true)))
        (Transformation|SetWorldLocationAndRotation _capsulecomponent (Math|Vector|MakeVector (.x _returnvalue) (.y _returnvalue) -2e+01) _returnvalue_2 false true)
        (Collision|SetCollisionResponsetoAllChannels _capsulecomponent "ECR_Ignore")
        (if (Variables|Default|GetIsTrainDeath)
          (Collision|SetCollisionResponsetoAllChannels _staticmesh "ECR_Overlap")
          (Transformation|SetWorldTransform _staticmesh (Math|Transform|MakeTransform (Math|Vector|MakeVector (.x _returnvalue) (.y _returnvalue) -2e+01) _returnvalue_2 "2.000000,2.000000,0.100000") false false)
          (Utilities|FlowControl|DoOnce false :!label _label
            (:Completed
              (Effects|SpawnEmitteratLocation "/Game/ParticleSystems/Feathers.Feathers" (Math|Vector|MakeVector (.x _returnvalue) (.y _returnvalue) 0.0))
              (Timeline|Wait%20After%20Death PlayFromStart
                (:Finished
                  (Default|DeathScreenin (Variables|Default|GetUI_Title))))))
          (elif (Variables|Default|GetIsDrownDeath)
            (Collision|SetCollisionResponsetoAllChannels _staticmesh "ECR_Overlap")
            (Transformation|SetWorldTransform _staticmesh (Math|Transform|MakeTransform (Math|Vector|MakeVector (.x _returnvalue) (.y _returnvalue) -2e+01) _returnvalue_2 "2.000000,2.000000,0.100000") false false)
            (Utilities|FlowControl|DoOnce false
              (:Completed
                (Effects|SpawnEmitteratLocation "/Game/ParticleSystems/Water.Water" (Math|Vector|MakeVector (.x _returnvalue) (.y _returnvalue) -2e+01))
                (Timeline|Wait%20After%20Death PlayFromStart)))
            (elif (Variables|Default|GetIsEagleDeath)
              (CallFunction|SpawntheEagle)
              (Collision|SetCollisionResponsetoAllChannels _staticmesh "ECR_Overlap")
              (Transformation|SetWorldTransform _staticmesh (Math|Transform|MakeTransform (Math|Vector|MakeVector (.x _returnvalue) (.y _returnvalue) -2e+01) "0, 0, 0" "2.000000,2.000000,0.100000") false false)
              (Utilities|FlowControl|DoOnce false
                (:Completed
                  (Effects|SpawnEmitteratLocation "/Game/ParticleSystems/Feathers.Feathers" (Math|Vector|MakeVector (.x _returnvalue) (.y _returnvalue) -2e+01))))
              (else
                (Collision|SetCollisionResponsetoAllChannels _staticmesh "ECR_Overlap")
                (Transformation|SetWorldTransform _staticmesh (Math|Transform|MakeTransform (Math|Vector|MakeVector (.x _returnvalue) (.y _returnvalue) 1.0) _returnvalue_2 "2.000000,2.000000,0.100000") false false)
                (goto _label)))))
        (else
          ;;[1 1 1] Do If Chicken Is Alive
          (Components|Activation|Deactivate (Variables|Default|GetFeathersExplosion))
          (Components|Activation|Deactivate (Variables|Default|GetWaterExplosion))
          (CallFunction|CameraMovement))))))

(event Collision|EventHit
  (params (MyComp :type Primitive%20Component%20Object%20Reference) (Other :type Actor%20Object%20Reference) (OtherComp :type Primitive%20Component%20Object%20Reference) (bSelfMoved :type Boolean) (HitLocation :type Vector :default "0, 0, 0") (HitNormal :type Vector :default "0, 0, 0") (NormalImpulse :type Vector :default "0, 0, 0") (Hit :type Hit%20Result%20Structure%20%28by%20ref%29))
  ;[1 1 1] Get/Set Chicken Death
  (if (Variables|Default|GetIsDead)
    _
    (else
      (Utilities|Casting|CastToBP_car1Left Other
        (:then
          _)
        (:CastFailed
          (if (Variables|Default|GetIsDead)
            _
            (else
              (Utilities|Casting|CastToBP_car1Right Other
                (:then
                  _)
                (:CastFailed
                  (if (Variables|Default|GetIsDead)
                    _
                    (else
                      (Utilities|Casting|CastToBP_car2Left Other
                        (:then
                          _)
                        (:CastFailed
                          (if (Variables|Default|GetIsDead)
                            _
                            (else
                              (Utilities|Casting|CastToBP_car2Right Other
                                (:then
                                  _)
                                (:CastFailed
                                  (if (Variables|Default|GetIsDead)
                                    _
                                    (else
                                      (Utilities|Casting|CastToBP_car3Left Other
                                        (:then
                                          _)
                                        (:CastFailed
                                          (if (Variables|Default|GetIsDead)
                                            _
                                            (else
                                              (Utilities|Casting|CastToBP_car3Right Other
                                                (:then
                                                  _)
                                                (:CastFailed
                                                  (if (Variables|Default|GetIsDead)
                                                    _
                                                    (else
                                                      (Utilities|Casting|CastToBP_truckLeft Other
                                                        (:then
                                                          _)
                                                        (:CastFailed
                                                          (if (Variables|Default|GetIsDead)
                                                            _
                                                            (else
                                                              (Utilities|Casting|CastToBP_truckRight Other
                                                                (:then
                                                                  _)
                                                                (:CastFailed
                                                                  (if (Variables|Default|GetIsDead)
                                                                    _
                                                                    (else
                                                                      (Utilities|Casting|CastToBP_trainLeft Other
                                                                        (:then
                                                                          _)
                                                                        (:CastFailed
                                                                          (if (Variables|Default|GetIsDead)
                                                                            _
                                                                            (else
                                                                              (Utilities|Casting|CastToBP_trainRight Other)))))))))))))))))))))))))))))))))))))))
  (Variables|Default|SetIsDead true))

(event EventBeginPlay
  ;[1 1 1] Camera Movement
  (Variables|Default|SetR_Forward (Transformation|GetWorldRotation (Variables|Default|GetStaticMesh)))
  (Transformation|SetAbsolute (Variables|Default|GetCamera) false false false)
  ;[1 1 1] Game Start Screen Creation
  (bind _returnvalue (UserInterface|CreateWidget "/Game/UI/UI.UI_C"))
  (bind _output_get (Variables|Default|SetUI_Title _returnvalue))
  (UserInterface|Viewport|AddtoViewport _output_get 0)
  (if (not (Variables|Default|GetGameStart))
    (Default|StartAnimationin (Variables|Default|GetUI_Title))
    (CallFunction|PlayTrafficSound)))

(event Input|ActionEvents|InputActionMoveForward
  (params (Key :type Key%20Structure))
  ;[1 1 1] Chicken Movement
  (:Pressed
    ;;[1 1 1] Title Animates Away When Player Starts
    (if (Variables|Default|GetGameStart)
      _
      (else
        (Default|StartAnimationOut (Variables|Default|GetUI_Title))
        (Variables|Default|SetGameStart true)))
    (bind _continue_ (CallFunction|CheckChickenFirst (Variables|Default|GetR_Forward)))
    (if _continue_
      (Variables|Default|SetChickenIsMoving true)
      (CallFunction|PlayCluckSound)
      (Timeline|Timeline_1 PlayFromStart
        (:Update
          (Character|Jump)
          (Transformation|AddWorldOffset (Variables|Collision|GetCapsuleComponent) (Math|Vector|MakeVector (* (Variables|Default|GetMaxSpeed%28-%29) (stale EventTick DeltaSeconds)) 0.0 0.0) true false))
        (:Finished
          (CallFunction|IncrementDistanceCounter)
          (Variables|Default|SetChickenIsMoving false)
          (Variables|Default|SetIdleTime 0))))))

(event Input|ActionEvents|InputActionMoveRight
  (params (Key :type Key%20Structure))
  ;[1 1 1] Chicken Movement
  (:Pressed
    (bind _continue_ (CallFunction|CheckChickenFirst (Variables|Default|GetR_Right)))
    (if _continue_
      (Variables|Default|SetChickenIsMoving true)
      (CallFunction|PlayCluckSound)
      (Timeline|Timeline_2 PlayFromStart
        (:Update
          (Character|Jump)
          (Transformation|AddWorldOffset (Variables|Collision|GetCapsuleComponent) (Math|Vector|MakeVector 0.0 (* (Variables|Default|GetMaxSpeed%28-%29) (stale EventTick DeltaSeconds)) 0.0) true false))
        (:Finished
          (Variables|Default|SetChickenIsMoving false)
          (Variables|Default|SetIdleTime 0))))))

(event Input|ActionEvents|InputActionMoveBack
  (params (Key :type Key%20Structure))
  ;[1 1 1] Chicken Movement
  (:Pressed
    (bind _continue_ (CallFunction|CheckChickenFirst (Variables|Default|GetR_Downward)))
    (if _continue_
      (Variables|Default|SetChickenIsMoving true)
      (CallFunction|PlayCluckSound)
      (Timeline|Timeline_3 PlayFromStart
        (:Update
          (Character|Jump)
          (Transformation|AddWorldOffset (Variables|Collision|GetCapsuleComponent) (Math|Vector|MakeVector (* (stale EventTick DeltaSeconds) (Variables|Default|GetMaxSpeed)) 0.0 0.0) true false))
        (:Finished
          (Variables|Default|SetChickenIsMoving false)
          (Variables|Default|SetIdleTime 0))))))

(event Input|ActionEvents|InputActionMoveLeft
  (params (Key :type Key%20Structure))
  ;[1 1 1] Chicken Movement
  (:Pressed
    (bind _continue_ (CallFunction|CheckChickenFirst (Variables|Default|GetR_Left)))
    (if _continue_
      (Variables|Default|SetChickenIsMoving true)
      (CallFunction|PlayCluckSound)
      (Timeline|Timeline_0 PlayFromStart
        (:Update
          (Character|Jump)
          (Transformation|AddWorldOffset (Variables|Collision|GetCapsuleComponent) (Math|Vector|MakeVector 0.0 (* (stale EventTick DeltaSeconds) (Variables|Default|GetMaxSpeed)) 0.0) true false))
        (:Finished
          (Variables|Default|SetChickenIsMoving false)
          (Variables|Default|SetIdleTime 0))))))

(fn ConstructionScript)

(fn CameraMovement
  (bind _staticmesh (Variables|Default|GetStaticMesh))
  (bind _springarm (Variables|Default|GetSpringArm))
  (bind _springarm_2 (Variables|Default|GetSpringArm))
  (bind _returnvalue (Transformation|GetWorldLocation _staticmesh))
  (bind _returnvalue_2 (Transformation|GetWorldLocation _springarm))
  ;[1 1 1] Y_Axis
  (if (< (.y _returnvalue) (.y _returnvalue_2))
    (Transformation|AddWorldOffset _springarm_2 (Math|Vector|MakeVector 0.0 -1e+01 0.0) true false)
    (elif (> (.y _returnvalue) (.y _returnvalue_2))
      (Transformation|AddWorldOffset _springarm_2 (Math|Vector|MakeVector 0.0 1e+01 0.0) true false)
      (else
        ;[1 1 1] X_Axis
        (if (<= (.x _returnvalue) (.x _returnvalue_2))
          (Transformation|AddWorldOffset _springarm_2 (Math|Vector|MakeVector -5.0 0.0 0.0) true false)
          (elif (> (.x _returnvalue) (.x _returnvalue_2))
            (Transformation|AddWorldOffset _springarm_2 (Math|Vector|MakeVector 5.0 0.0 0.0) true false)))))))

(fn IstheChickenMid-Jump
  (if (or (Character|IsJumpProvidingForce) (AI|Components|NavMovement|IsFalling (Variables|Character|GetCharacterMovement)))
    (Variables|Default|SetIsMidJump true)
    (else
      (Variables|Default|SetIsMidJump false))))

(fn IncrementDistanceCounter
  (if (not (Variables|Default|GetIsDead))
    (bind _result (Math|Integer|IncrementInt (Variables|Default|GetChickenDistance))
      (:%20%20
        (Default|UpdateDistance (Variables|Default|GetUI_Title) _result)))))

(fn CheckChickenFirst
  (params (RotationToCompare :type Rotator))
  (bind _staticmesh (Variables|Default|GetStaticMesh))
  (if (Variables|Default|GetIsDead)
    _
    (elif (Variables|Default|GetisBlockedLeft)
      _
      (elif (Variables|Default|GetisBlockedRight)
        _
        (else
          (if (Math|Rotator|Equal(Rotator) (Transformation|GetWorldRotation _staticmesh) RotationToCompare 0.1)
            (if (Variables|Default|GetIsMidJump)
              (return false false)
              (else
                _))
            (else
              (Transformation|SetWorldRotation _staticmesh RotationToCompare false false)))
          (Variables|Default|SetPreviousSpot (Transformation|GetWorldLocation (Variables|Collision|GetCapsuleComponent)))
          (return true false)))))
  (return false true))

(fn PlayCluckSound
  (Audio|Components|Audio|SetSound (Variables|Default|GetCluckSound) "/Game/Sounds/Chickendeepcluckbasicjump.Chickendeepcluckbasicjump")
  (Audio|SpawnSoundAttached "/Game/Sounds/Chickendeepcluckbasicjump.Chickendeepcluckbasicjump" (Variables|Default|GetStaticMesh) "None" "0, 0, 0" "0, 0, 0" "KeepRelativeOffset" false 1.0 1.0 0.0 0 0))

(fn ChickenWorldBoundCheck)

(fn PutChickenBackinBounds
  (Transformation|SetWorldLocation (Variables|Collision|GetCapsuleComponent) (Variables|Default|GetPreviousSpot) false false)
  (Variables|Default|SetisBlockedLeft false)
  (Variables|Default|SetisBlockedRight false))

(fn IncrementCoinsCollected
  (bind _result (Math|Integer|IncrementInt (Variables|Default|GetCoinsCollected))
    (:%20%20
      (Default|UpdateCoins (Variables|Default|GetUI_Title) _result))))

(fn PlayDeathSound
  (Audio|Components|Audio|SetSound (Variables|Default|GetDeathSound) "/Game/Sounds/ChickenCluck.ChickenCluck")
  (Audio|SpawnSoundAttached "/Game/Sounds/ChickenCluck.ChickenCluck" (Variables|Default|GetStaticMesh) "None" "0, 0, 0" "0, 0, 0" "KeepRelativeOffset" false 1.0 1.0 0.0 0 0))

(fn PlayTrafficSound
  (Audio|Components|Audio|SetSound (Variables|Default|GetTrafficNoise) "/Game/Sounds/TrafficNoise.TrafficNoise")
  (Audio|SpawnSoundAttached "/Game/Sounds/TrafficNoise.TrafficNoise" (Variables|Default|GetStaticMesh) "None" "0, 0, 0" "0, 0, 0" "KeepRelativeOffset" false 1.0 1.0 0.0 0 0))

(fn SpawntheEagle)