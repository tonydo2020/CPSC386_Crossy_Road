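; Truck obstacle that drives along the world Y axis and kills the chicken character on contact.
; BeginPlay sets a fixed rotation and stores the mesh's start location, then Tick moves the actor with a swept offset scaled by ForwardSpeed.
; Once the mesh passes a hard-coded negative Y limit, the mesh component, not the actor, moves back to the start.
; Mesh hits on BPC_Chicken set its IsDead flag.
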(event OnComponentHit(StaticMesh)
  (params (HitComponent :type Primitive%20Component%20Object%20Reference) (OtherActor :type Actor%20Object%20Reference) (OtherComp :type Primitive%20Component%20Object%20Reference) (NormalImpulse :type Vector :default "0, 0, 0") (Hit :type Hit%20Result%20Structure%20%28by%20ref%29))
  (bind _asbpc_chicken (Utilities|Casting|CastToBPC_Chicken OtherActor))
  (Variables|/Game/Blueprints/BPC_Chicken.BPC_Chicken_C|SetIsDead _asbpc_chicken true))

(event EventBeginPlay
  (Transformation|SetActorRotation "0,180.000000, 0")
  (Variables|Default|SetStartingPoint (Transformation|GetWorldLocation (Variables|Default|GetStaticMesh))))

(event EventTick
  (params (DeltaSeconds :type Float%20%28single-precision%29))
  (if (< (.y (Transformation|GetWorldLocation (Variables|Default|GetStaticMesh))) -2e+03)
    (Transformation|SetWorldLocation (Variables|Default|GetStaticMesh) (Variables|Default|GetStartingPoint) false false)
    (else
      (Transformation|AddActorWorldOffset (Math|Vector|MakeVector 0.0 (* DeltaSeconds (Variables|Default|Getforward_speed)) 0.0) true))))

(fn ConstructionScript)