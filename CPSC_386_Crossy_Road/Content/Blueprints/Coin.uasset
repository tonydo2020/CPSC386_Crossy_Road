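; Coin pickup actor that the BPC_Chicken character collects on touch.
; When the chicken overlaps the collision box, the box ignores all channels so it cannot trigger again, and the coin component drops to a negative world Z rather than being destroyed.
; It then plays the coin sound at that location and calls IncrementCoinsCollected on the chicken.
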(event OnComponentBeginOverlap(CollisionBox)
  (params (OverlappedComponent :type Primitive%20Component%20Object%20Reference) (OtherActor :type Actor%20Object%20Reference) (OtherComp :type Primitive%20Component%20Object%20Reference) (OtherBodyIndex :type Integer) (bFromSweep :type Boolean) (SweepResult :type Hit%20Result%20Structure%20%28by%20ref%29))
  (bind _coin (Variables|Default|GetCoin))
  (bind _returnvalue (Transformation|GetWorldLocation _coin))
  (bind _asbpc_chicken (Utilities|Casting|CastToBPC_Chicken OtherActor))
  (Collision|SetCollisionResponsetoAllChannels (Variables|Default|GetCollisionBox) "ECR_Ignore")
  (Transformation|SetWorldLocation (Variables|Default|GetCoin) (Math|Vector|MakeVector (.x _returnvalue) (.y _returnvalue) -1e+01) false false)
  (Audio|PlaySoundatLocation "/Game/Sounds/Coin.Coin" (Transformation|GetWorldLocation (Variables|Default|GetCoin)) "0, 0, 0" 1.0 1.0 0.0 0 0 0)
  (Default|IncrementCoinsCollected _asbpc_chicken))

(event EventBeginPlay)

(event Collision|EventActorBeginOverlap
  (params (OtherActor :type Actor%20Object%20Reference)))

(event EventTick
  (params (DeltaSeconds :type Float%20%28single-precision%29)))

(fn ConstructionScript)