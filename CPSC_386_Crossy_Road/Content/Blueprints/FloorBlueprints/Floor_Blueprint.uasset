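; Floor tile Blueprint that reacts to the chicken character (BPC_Chicken) through three overlap volumes.
; Entering TriggerZone tells the FloorSpawner to spawn a floor at its spawn point, extending the ground.
; DespawnLeft and DespawnRight both set the chicken's IsBlockedLeft flag on overlap, despite their names.
; The nodes that clear the flag are unconnected, so this asset never resets it.
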(event OnComponentBeginOverlap(DespawnLeft)
  (params (OverlappedComponent :type Primitive%20Component%20Object%20Reference) (OtherActor :type Actor%20Object%20Reference) (OtherComp :type Primitive%20Component%20Object%20Reference) (OtherBodyIndex :type Integer) (bFromSweep :type Boolean) (SweepResult :type Hit%20Result%20Structure%20%28by%20ref%29))
  (bind _asbpc_chicken (Utilities|Casting|CastToBPC_Chicken OtherActor))
  (Variables|/Game/Blueprints/BPC_Chicken.BPC_Chicken_C|SetisBlockedLeft _asbpc_chicken true))

(event OnComponentBeginOverlap(TriggerZone)
  (params (OverlappedComponent :type Primitive%20Component%20Object%20Reference) (OtherActor :type Actor%20Object%20Reference) (OtherComp :type Primitive%20Component%20Object%20Reference) (OtherBodyIndex :type Integer) (bFromSweep :type Boolean) (SweepResult :type Hit%20Result%20Structure%20%28by%20ref%29))
  (Utilities|Casting|CastToBPC_Chicken OtherActor)
  (Default|SpawnFlooratSpawnPoint (Variables|Default|GetFloorSpawner)))

(event OnComponentBeginOverlap(DespawnRight)
  (params (OverlappedComponent :type Primitive%20Component%20Object%20Reference) (OtherActor :type Actor%20Object%20Reference) (OtherComp :type Primitive%20Component%20Object%20Reference) (OtherBodyIndex :type Integer) (bFromSweep :type Boolean) (SweepResult :type Hit%20Result%20Structure%20%28by%20ref%29))
  (bind _asbpc_chicken (Utilities|Casting|CastToBPC_Chicken OtherActor))
  (Variables|/Game/Blueprints/BPC_Chicken.BPC_Chicken_C|SetisBlockedLeft _asbpc_chicken true))

(event EventBeginPlay)

(fn ConstructionScript)