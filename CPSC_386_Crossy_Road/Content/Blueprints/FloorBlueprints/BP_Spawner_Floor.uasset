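; Spawner that builds a chain of random floor tiles (grass, river, railroad) from the player's location.
; On BeginPlay it lays starting grass, then appends floors at the newest tile's SpawnPoint, giving each a reference back to the spawner.
; Only Easy selection is wired, randomly excluding the first list entry to make it rarer.
; True-random Hard is disconnected, Medium is empty, and SpawnTrees is not called here.
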(event EventBeginPlay
  (CallFunction|SpawnInitialFloors))

(event Collision|EventActorBeginOverlap
  (params (OtherActor :type Actor%20Object%20Reference)))

(event EventTick
  (params (DeltaSeconds :type Float%20%28single-precision%29)))

(fn ConstructionScript)

(fn SpawnFloorDifficulty
  (params (SpawnLocation :type Vector))
  (CallFunction|SpawnFloorEasy(LessRiver/Railroad) SpawnLocation))

(fn SpawnFlooratSpawnPoint
  (CallFunction|SpawnFloorDifficulty (Transformation|GetWorldLocation (Variables|/Game/Blueprints/FloorBlueprints/Floor_Blueprint.Floor_Blueprint_C|GetSpawnPoint (Variables|Default|GetNewestFloor)))))

(fn SpawnInitialFloors
  (for _index (range 0 10)
    (Utilities|IsValid (Variables|Default|GetNewestFloor)
      (:Is%20Valid
        (CallFunction|SpawnFlooratSpawnPoint))
      (:Is%20Not%20Valid
        (CallFunction|SpawnStartingGrasses)))))

(fn SpawnTrees
  (bind _newestfloor (Variables|Default|GetNewestFloor))
  (bind _spawnpoint (Variables|/Game/Blueprints/FloorBlueprints/Floor_Blueprint.Floor_Blueprint_C|GetSpawnPoint _newestfloor))
  (bind _returnvalue (Transformation|GetWorldLocation _spawnpoint))
  (for _index (range 1 5)
    (Game|SpawnActorfromClass "/Game/Blueprints/BP_treeT.BP_treeT_C" (Math|Transform|MakeTransform (Math|Vector|MakeVector (+ (Math|Random|RandomFloatinRange 1.0 2e+02) (.y _returnvalue)) (.x _returnvalue) 0.0) "0, 0, 0" "1,1,1") "Undefined" 0 0)))

(fn SpawnStartingGrasses
  (bind _returnvalue (Game|SpawnActorfromClass "/Game/Blueprints/FloorBlueprints/FloorCh_Grass.FloorCh_Grass_C" (Math|Transform|MakeTransform (Transformation|GetActorLocation (Game|GetPlayerCharacter 0)) "0,-90.000000, 0" "1,1,1") "Undefined" 0 0))
  (bind _output_get (Variables|Default|SetNewestFloor _returnvalue))
  (Variables|/Game/Blueprints/FloorBlueprints/Floor_Blueprint.Floor_Blueprint_C|SetFloorSpawner _output_get self)
  (for _index (range 0 1)
    (bind _returnvalue_2 (Game|SpawnActorfromClass "/Game/Blueprints/FloorBlueprints/FloorCh_Grass.FloorCh_Grass_C" (Math|Transform|MakeTransform (Transformation|GetWorldLocation (Variables|/Game/Blueprints/FloorBlueprints/Floor_Blueprint.Floor_Blueprint_C|GetSpawnPoint (Variables|Default|GetNewestFloor))) "0,-90.000000, 0" "1,1,1") "Undefined" 0 0))
    (bind _asfloor_blueprint (Utilities|Casting|CastToFloor_Blueprint _returnvalue_2))
    (bind _output_get_2 (Variables|Default|SetNewestFloor _asfloor_blueprint))
    (Variables|/Game/Blueprints/FloorBlueprints/Floor_Blueprint.Floor_Blueprint_C|SetFloorSpawner _output_get_2 self)))

(fn SpawnFloorHard(TrueRandom)
  (params (Location :type Vector))
  (bind _list_of_actors (Variables|Default|GetList%20of%20Actors))
  (bind _returnvalue (Game|SpawnActorfromClass (Utilities|Array|Get(acopy) _list_of_actors (Math|Random|RandomIntegerinRange 0 (Utilities|Array|LastIndex _list_of_actors))) (Math|Transform|MakeTransform Location "0,-90.000000, 0" "1,1,1") "Undefined" 0 0))
  (bind _asfloor_blueprint (Utilities|Casting|CastToFloor_Blueprint _returnvalue))
  (bind _output_get (Variables|Default|SetNewestFloor _asfloor_blueprint))
  (Variables|/Game/Blueprints/FloorBlueprints/Floor_Blueprint.Floor_Blueprint_C|SetFloorSpawner _output_get self))

(fn SpawnFloorEasy(LessRiver/Railroad)
  (params (Location :type Vector))
  (bind _list_of_actors (Variables|Default|GetList%20of%20Actors))
  (bind _returnvalue (Game|SpawnActorfromClass (Utilities|Array|Get(acopy) _list_of_actors (Math|Random|RandomIntegerinRange (Math|Conversions|ToInteger(Boolean) (Math|Random|RandomBool)) (Utilities|Array|LastIndex _list_of_actors))) (Math|Transform|MakeTransform Location "0,-90.000000, 0" "1,1,1") "Undefined" 0 0))
  (bind _asfloor_blueprint (Utilities|Casting|CastToFloor_Blueprint _returnvalue))
  (bind _output_get (Variables|Default|SetNewestFloor _asfloor_blueprint))
  (Variables|/Game/Blueprints/FloorBlueprints/Floor_Blueprint.Floor_Blueprint_C|SetFloorSpawner _output_get self))

(fn SpawnFloorMedium
  (params (Location :type Vector)))