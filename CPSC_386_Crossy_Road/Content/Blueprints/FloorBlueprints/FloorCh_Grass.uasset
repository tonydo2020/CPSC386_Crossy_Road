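; Grass floor tile Blueprint that populates itself with boundary trees, scattered props and a coin when play begins.
; Fixed scene-component markers place single trees and three-tree clusters on both sides.
; A loop spawns random props from ListOfObjects at a random Y in a left or right band along the marker's X line, skipping any that cannot avoid collision.
; One coin always spawns at a random Y between the despawn markers.
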(event EventBeginPlay
  (|CallParentFunction)
  (CallFunction|SpawnBoundaryTrees)
  (CallFunction|SpawnRocks/Bushes/Trees)
  (CallFunction|SpawnCoins))

(event Collision|EventActorBeginOverlap
  (params (OtherActor :type Actor%20Object%20Reference)))

(event EventTick
  (params (DeltaSeconds :type Float%20%28single-precision%29)))

(fn ConstructionScript
  (|CallParentFunction))

(fn SpawnBoundaryTrees
  (Game|SpawnActorfromClass "/Game/Blueprints/BP_treeT.BP_treeT_C" (Math|Transform|MakeTransform (Transformation|GetWorldLocation (Variables|Default|GetSpawnRight)) "0, 0, 0" "1,1,1") "Undefined" 0 0)
  (Game|SpawnActorfromClass "/Game/Blueprints/BP_treeT.BP_treeT_C" (Math|Transform|MakeTransform (Transformation|GetWorldLocation (Variables|Default|GetSpawnLeft)) "0, 0, 0" "1,1,1") "Undefined" 0 0)
  (Game|SpawnActorfromClass "/Game/Blueprints/BP_3trees.BP_3trees_C" (Math|Transform|MakeTransform (Transformation|GetWorldLocation (Variables|Default|GetTree%20Limit%20Left)) "0, 0, 0" "1,1,1") "Undefined" 0 0)
  (Game|SpawnActorfromClass "/Game/Blueprints/BP_3trees.BP_3trees_C" (Math|Transform|MakeTransform (Transformation|GetWorldLocation (Variables|Default|GetTree%20Boundary%20Right)) "0, 0, 0" "1,1,1") "Undefined" 0 0))

(fn SpawnRocks/Bushes/Trees
  (bind _returnvalue (Math|Random|RandomBool))
  (bind _listofobjects (Variables|Default|GetListOfObjects))
  (bind _spawnleft (Variables|Default|GetSpawnLeft))
  (bind _returnvalue_2 (Transformation|GetWorldLocation _spawnleft))
  (for _index (range 0 4)
    (Game|SpawnActorfromClass (Utilities|Array|Get(acopy) _listofobjects (Math|Random|RandomIntegerinRange (Math|Conversions|ToInteger(Boolean) _returnvalue) (Utilities|Array|LastIndex _listofobjects))) (Math|Transform|MakeTransform (Math|Vector|MakeVector (.x _returnvalue_2) (select _returnvalue (Math|Random|RandomFloatinRange (Variables|Default|Gety_playerspawnbound_left) (.y (Transformation|GetWorldLocation (Variables|Default|GetSpawnLeft)))) (Math|Random|RandomFloatinRange (.y (Transformation|GetWorldLocation (Variables|Default|GetSpawnRight))) (Variables|Default|Gety_playerspawnbound_right))) (.z _returnvalue_2)) "0, 0, 0" "1,1,1") "AdjustIfPossibleButDontSpawnIfColliding" 0 0)))

(fn SpawnCoins
  (bind _spawnright (Variables|Default|GetSpawnRight))
  (bind _returnvalue (Transformation|GetWorldLocation _spawnright))
  (Game|SpawnActorfromClass "/Game/Blueprints/Coin.Coin_C" (Math|Transform|MakeTransform (Math|Vector|MakeVector (.x _returnvalue) (Math|Random|RandomFloatinRange (.y (Transformation|GetWorldLocation (Variables|Default|GetDespawnRight))) (.y (Transformation|GetWorldLocation (Variables|Default|GetDespawnLeft)))) (.z _returnvalue)) "0, 0, 0" "1,1,1") "AdjustIfPossibleButAlwaysSpawn" 0 0))