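; Road floor chunk Blueprint that spawns a single moving-traffic car when play begins.
; On BeginPlay it randomly spawns immediately or first waits for one of two timelines to finish, using them as delays to stagger traffic.
; A coin flip picks the direction, then a random class from that direction's array spawns at the opposite side's spawn point and is stored.
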(event EventBeginPlay
  (bind _carsgoingleft (Variables|Default|GetCarsGoingLeft))
  (bind _carsgoingright (Variables|Default|GetCarsGoingRight))
  (|CallParentFunction)
  (switch int (Math|Random|RandomIntegerinRange 0 2)
    (:0
      (Timeline|Timeline_0 PlayFromStart
        (:Finished
          _)))
    (:1
      (Timeline|Timeline_1 PlayFromStart
        (:Finished
          _)))
    (:2
      _))
  (if (Math|Random|RandomBool)
    (bind _returnvalue (Game|SpawnActorfromClass (Utilities|Array|Get(acopy) _carsgoingright (Math|Random|RandomIntegerinRange 0 (Utilities|Array|LastIndex _carsgoingright))) (Math|Transform|MakeTransform (Transformation|GetWorldLocation (Variables|Default|GetSpawnLeft)) "0, 0, 0" "1,1,1") "AdjustIfPossibleButAlwaysSpawn" 0 0))
    (Variables|Default|SetCarGoingRight _returnvalue)
    (else
      (bind _returnvalue_2 (Game|SpawnActorfromClass (Utilities|Array|Get(acopy) _carsgoingleft (Math|Random|RandomIntegerinRange 0 (Utilities|Array|LastIndex _carsgoingleft))) (Math|Transform|MakeTransform (Transformation|GetWorldLocation (Variables|Default|GetSpawnRight)) "0, 0, 0" "1,1,1") "AdjustIfPossibleButAlwaysSpawn" 0 0))
      (Variables|Default|SetCarGoingLeft _returnvalue_2))))

(fn ConstructionScript
  (|CallParentFunction))