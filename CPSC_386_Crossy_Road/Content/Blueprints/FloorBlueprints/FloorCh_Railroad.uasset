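; Railroad crossing floor piece that sends trains across it, starting in a random direction after a timeline delay on BeginPlay.
; Each spawn coincides with a warning sound and alternately flashing lights, and DespawnLeft/Right overlaps play the passing sound.
; DespawnTrainLeft/Right overlaps call destroy on the opposite direction's train reference, not the overlapping train, then respawn the same direction after a delay.
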(event OnComponentBeginOverlap(DespawnLeft)
  (params (OverlappedComponent :type Primitive%20Component%20Object%20Reference) (OtherActor :type Actor%20Object%20Reference) (OtherComp :type Primitive%20Component%20Object%20Reference) (OtherBodyIndex :type Integer) (bFromSweep :type Boolean) (SweepResult :type Hit%20Result%20Structure%20%28by%20ref%29))
  (Utilities|Casting|CastToBP_trainRight OtherActor)
  (CallFunction|PlayTrainPassing))

(event OnComponentBeginOverlap(DespawnRight)
  (params (OverlappedComponent :type Primitive%20Component%20Object%20Reference) (OtherActor :type Actor%20Object%20Reference) (OtherComp :type Primitive%20Component%20Object%20Reference) (OtherBodyIndex :type Integer) (bFromSweep :type Boolean) (SweepResult :type Hit%20Result%20Structure%20%28by%20ref%29))
  (Utilities|Casting|CastToBP_trainLeft OtherActor)
  (CallFunction|PlayTrainPassing))

(event OnComponentBeginOverlap(DespawnTrainLeft)
  (params (OverlappedComponent :type Primitive%20Component%20Object%20Reference) (OtherActor :type Actor%20Object%20Reference) (OtherComp :type Primitive%20Component%20Object%20Reference) (OtherBodyIndex :type Integer) (bFromSweep :type Boolean) (SweepResult :type Hit%20Result%20Structure%20%28by%20ref%29))
  (Utilities|Casting|CastToBP_trainLeft OtherActor)
  (Actor|DestroyActor (Variables|Default|GetTrainGoingRight))
  (Timeline|3sec_2 PlayFromStart
    (:Finished
      (CallFunction|TrainWarning)
      (CallFunction|SpawnTrain false))))

(event OnComponentBeginOverlap(DespawnTrainRight)
  (params (OverlappedComponent :type Primitive%20Component%20Object%20Reference) (OtherActor :type Actor%20Object%20Reference) (OtherComp :type Primitive%20Component%20Object%20Reference) (OtherBodyIndex :type Integer) (bFromSweep :type Boolean) (SweepResult :type Hit%20Result%20Structure%20%28by%20ref%29))
  (Utilities|Casting|CastToBP_trainRight OtherActor)
  (Actor|DestroyActor (Variables|Default|GetTrainGoingLeft))
  (Timeline|3sec_1 PlayFromStart
    (:Finished
      (CallFunction|TrainWarning)
      (CallFunction|SpawnTrain true))))

(event Custom|TrainWarning
  (bind _trainlight1 (Variables|Default|GetTrainLight1))
  (bind _trainlight2 (Variables|Default|GetTrainLight2))
  (bind _trainlight2_2 (Variables|Default|GetTrainLight2))
  (bind _trainlight1_2 (Variables|Default|GetTrainLight1))
  (bind _trainlight2_3 (Variables|Default|GetTrainLight2))
  (bind _trainlight1_3 (Variables|Default|GetTrainLight1))
  ;[1 1 1] Train Warning
  (CallFunction|PlayTrainWarning)
  (Rendering|ToggleVisibility _trainlight2_2 false)
  (Utilities|FlowControl|Delay 0.3)
  (Rendering|ToggleVisibility _trainlight2_2 false)
  (Rendering|ToggleVisibility _trainlight1_2 false)
  (Utilities|FlowControl|Delay 0.3)
  (Rendering|ToggleVisibility _trainlight1_2 false)
  (Rendering|ToggleVisibility _trainlight2_3 false)
  (Utilities|FlowControl|Delay 0.3)
  (Rendering|ToggleVisibility _trainlight2_3 false)
  (Rendering|ToggleVisibility _trainlight1_3 false)
  (Utilities|FlowControl|Delay 0.3)
  (Rendering|ToggleVisibility _trainlight1_3 false)
  (Rendering|ToggleVisibility _trainlight2 false)
  (Utilities|FlowControl|Delay 0.3)
  (Rendering|ToggleVisibility _trainlight2 false)
  (Rendering|ToggleVisibility _trainlight1 false)
  (Utilities|FlowControl|Delay 0.3)
  (Rendering|ToggleVisibility _trainlight1 false)
  (Utilities|FlowControl|Delay 2.0))

(event EventBeginPlay
  (|CallParentFunction)
  (Timeline|3Sec_3 PlayFromStart
    (:Finished
      (CallFunction|TrainWarning)
      (Development|PrintString "Spawning Train")
      (CallFunction|SpawnTrain (Math|Random|RandomBool)))))

(fn ConstructionScript
  (|CallParentFunction))

(fn PlayTrainPassing
  (Audio|Components|Audio|SetSound (Variables|Default|GetTrainWarningBell) "/Game/Sounds/TrainPassing.TrainPassing")
  (Audio|SpawnSoundAttached "/Game/Sounds/TrainPassing.TrainPassing" (Variables|Default|GetTrainPost) "None" "0, 0, 0" "0, 0, 0" "KeepRelativeOffset" false 1.0 1.0 0.0 0 0))

(fn SpawnTrain
  (params (RightOrLeft :type Boolean))
  (if RightOrLeft
    (bind _returnvalue (Game|SpawnActorfromClass "/Game/Blueprints/Vehicle_BP/BP_trainRight.BP_trainRight_C" (Math|Transform|MakeTransform (Transformation|GetWorldLocation (Variables|Default|GetSpawnLeft)) "0, 0, 0" "0.750000,1.000000,1") "AdjustIfPossibleButAlwaysSpawn" 0 0))
    (Variables|Default|SetTrainGoingRight _returnvalue)
    (else
      (bind _returnvalue_2 (Game|SpawnActorfromClass "/Game/Blueprints/Vehicle_BP/BP_trainLeft.BP_trainLeft_C" (Math|Transform|MakeTransform (Transformation|GetWorldLocation (Variables|Default|GetSpawnRight)) "0, 0, 0" "0.750000,1,1") "AdjustIfPossibleButAlwaysSpawn" 0 0))
      (Variables|Default|SetTrainGoingLeft _returnvalue_2))))

(fn PlayTrainWarning
  (Audio|Components|Audio|SetSound (Variables|Default|GetTrainWarningBell) "/Game/Sounds/TrainWarning.TrainWarning")
  (Audio|SpawnSoundAttached "/Game/Sounds/TrainWarning.TrainWarning" (Variables|Default|GetTrainPost) "None" "0, 0, 0" "0, 0, 0" "KeepRelativeOffset" false 1.0 1.0 0.0 0 0))