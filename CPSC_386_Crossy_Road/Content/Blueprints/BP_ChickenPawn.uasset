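; BP_ChickenPawn is a player pawn for a chicken that moves in fixed world-space steps from four directional input actions.
; A press either turns the chicken to that direction or, when it already faces that way, moves it one step without sweeping for collision.
; Facing is inferred by comparing actor rotation to stored rotators.
; BeginPlay captures only the forward rotator from the starting rotation, and the graph never sets the others.
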(event Collision|EventActorBeginOverlap
  (params (OtherActor :type Actor%20Object%20Reference)))

(event EventTick
  (params (DeltaSeconds :type Float%20%28single-precision%29)))

(event EventBeginPlay
  (Variables|Default|SetR_Forward (Transformation|GetActorRotation)))

(event Input|ActionEvents|InputActionMoveForward
  (params (Key :type Key%20Structure))
  (:Pressed
    (if (Math|Rotator|Equal(Rotator) (Transformation|GetActorRotation) (Variables|Default|GetR_Forward) 0.0001)
      (Transformation|AddActorWorldOffset "-200.000000,0.000000, 0")
      (else
        (Transformation|SetActorRelativeRotation (Variables|Default|GetR_Forward))))))

(event Input|ActionEvents|InputActionMoveBack
  (params (Key :type Key%20Structure))
  (:Pressed
    (if (Math|Rotator|Equal(Rotator) (Transformation|GetActorRotation) (Variables|Default|GetR_Forward) 0.0001)
      (Transformation|SetActorRelativeRotation "0, 0, 0")
      (elif (Math|Rotator|Equal(Rotator) (Transformation|GetActorRotation) (Variables|Default|GetR_Left) 0.0001)
        (Transformation|SetActorRelativeRotation "0, 0, 0")
        (elif (Math|Rotator|Equal(Rotator) (Transformation|GetActorRotation) (Variables|Default|GetR_Right) 0.0001)
          (Transformation|SetActorRelativeRotation "0, 0, 0")
          (else
            (Transformation|AddActorWorldOffset "200.000000,0.000000, 0")))))))

(event Input|ActionEvents|InputActionMoveRight
  (params (Key :type Key%20Structure))
  (:Pressed
    (if (Math|Rotator|Equal(Rotator) (Transformation|GetActorRotation) (Variables|Default|GetR_Forward) 0.0001)
      (Transformation|SetActorRelativeRotation "0,-90.000000, 0")
      (elif (Math|Rotator|Equal(Rotator) (Transformation|GetActorRotation) (Variables|Default|GetR_Downward) 0.0001)
        (Transformation|SetActorRelativeRotation "0,-90.000000, 0")
        (elif (Math|Rotator|Equal(Rotator) (Transformation|GetActorRotation) (Variables|Default|GetR_Left) 0.0001)
          (Transformation|SetActorRelativeRotation "0,-90.000000, 0")
          (else
            (Transformation|AddActorWorldOffset "0.000000,-200.000000, 0")))))))

(event Input|ActionEvents|InputActionMoveLeft
  (params (Key :type Key%20Structure))
  (:Pressed
    (if (Math|Rotator|Equal(Rotator) (Transformation|GetActorRotation) (Variables|Default|GetR_Forward) 0.0001)
      (Transformation|SetActorRelativeRotation "0,90.000000, 0")
      (elif (Math|Rotator|Equal(Rotator) (Transformation|GetActorRotation) (Variables|Default|GetR_Downward) 0.0001)
        (Transformation|SetActorRelativeRotation "0,90.000000, 0")
        (elif (Math|Rotator|Equal(Rotator) (Transformation|GetActorRotation) (Variables|Default|GetR_Right) 0.0001)
          (Transformation|SetActorRelativeRotation "0,90.000000, 0")
          (else
            (Transformation|AddActorWorldOffset "0.000000,200.000000, 0")))))))

(fn ConstructionScript)