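; BP_logLeft is a moving log actor that travels along positive world Y and loops back to where it started.
; BeginPlay stores the static mesh's world location as the starting point.
; Each Tick offsets the actor by ForwardSpeed scaled by delta time until the mesh's Y reaches a hard-coded limit.
; At that limit it teleports only the mesh component back to the start, not the actor.
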(event EventTick
  (params (DeltaSeconds :type Float%20%28single-precision%29))
  (if (>= (.y (Transformation|GetWorldLocation (Variables|Default|GetStaticMesh))) 2e+03)
    (Transformation|SetWorldLocation (Variables|Default|GetStaticMesh) (Variables|Default|GetStartingPoint) false true)
    (else
      (Transformation|AddActorWorldOffset (Math|Vector|MakeVector 0.0 (* DeltaSeconds (Variables|Default|Getforward%20speed)) 0.0)))))

(event EventBeginPlay
  (Variables|Default|SetStartingPoint (Transformation|GetWorldLocation (Variables|Default|GetStaticMesh))))

(fn ConstructionScript)