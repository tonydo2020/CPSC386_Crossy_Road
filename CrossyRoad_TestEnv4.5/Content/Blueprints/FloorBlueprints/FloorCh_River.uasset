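; River floor tile for a chicken-crossing game that drowns any chicken hitting its water mesh.
; On BeginPlay it randomly spawns either a log or a set of lily pads.
; The log's direction is random, with its class and spawn side chosen to match.
; Lily pads get random Y positions between two limit markers, adjusting or skipping spawns that would collide.
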(event OnComponentHit(StaticMeshComponent)
  (params (HitComponent :type Primitive%20Component%20Object%20Reference) (OtherActor :type Actor%20Object%20Reference) (OtherComp :type Primitive%20Component%20Object%20Reference) (NormalImpulse :type Vector :default "0, 0, 0") (Hit :type Hit%20Result%20Structure%20%28by%20ref%29))
  (bind _asbpc_chicken (Utilities|Casting|CastToBPC_Chicken OtherActor))
  (Variables|/Game/Blueprints/BPC_Chicken.BPC_Chicken_C|SetIsDead _asbpc_chicken true)
  (Variables|/Game/Blueprints/BPC_Chicken.BPC_Chicken_C|SetIsDrownDeath _asbpc_chicken true))

(event EventBeginPlay
  (|CallParentFunction)
  (if (Math|Random|RandomBool)
    (CallFunction|SpawnLogs)
    (else
      (CallFunction|SpawnLilyPads))))

(fn ConstructionScript
  (|CallParentFunction))

(fn SpawnLogs
  (if (Math|Random|RandomBool)
    (bind _returnvalue (Game|SpawnActorfromClass "/Game/Blueprints/BP_logRight.BP_logRight_C" (Math|Transform|MakeTransform (Transformation|GetWorldLocation (Variables|Default|GetSpawnLeft)) "0,90.000000, 0" "2.000000,2.500000,1") "Undefined" 0 0))
    (Variables|Default|SetLogGoingRight _returnvalue)
    (else
      (bind _returnvalue_2 (Game|SpawnActorfromClass "/Game/Blueprints/BP_logLeft.BP_logLeft_C" (Math|Transform|MakeTransform (Transformation|GetWorldLocation (Variables|Default|GetSpawnRight)) "0,90.000000, 0" "2.000000,2.500000,1") "Undefined" 0 0))
      (Variables|Default|SetLogGoingLeft _returnvalue_2))))

(fn SpawnLilyPads
  (for _index (range 0 2)
    (Game|SpawnActorfromClass "/Game/Blueprints/Lily_Pad.Lily_Pad_C" (Math|Transform|MakeTransform (Math|Vector|MakeVector (.x (Transformation|GetWorldLocation (Variables|Default|GetSpawnLeft))) (Math|Random|RandomFloatinRange (.y (Transformation|GetWorldLocation (Variables|Default|GetLilyLimitRight))) (.y (Transformation|GetWorldLocation (Variables|Default|GetLilyLimitLeft)))) 2.0) "0, 0, 0" "1.500000,1.500000,2.000000") "AdjustIfPossibleButDontSpawnIfColliding" 0 0)))